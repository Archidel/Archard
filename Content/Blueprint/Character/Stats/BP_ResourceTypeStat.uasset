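; BP_ResourceTypeStat is a character stat Blueprint for a resource-type value bounded by MinValue and MaxValue.
; ChangeValue checks that the StatsManager's ResourceStat is valid, then switches on an Add, Reduce or Change action and clamps the result.
; Reaching a bound through these actions fires ValueIsMax or ValueIsMin, which currently only print debug strings.
; RegenerationResource is an empty stub.
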(event `self.ValueIsMax`
  (`KismetSystemLibrary.PrintString` "Max"))

(event `self.ValueIsMin`
  (`KismetSystemLibrary.PrintString` "Min"))

(event `self.ChangeValue`
  (params (Value :type "Float (single-precision)") (Action :type "/Game/Enum/Support/E_Method_Action Enum" :default "NewEnumerator0"))
  (bind _returnvalue (- (`self.Value`) Value))
  (bind _returnvalue_2 (+ (`self.Value`) Value))
  (`/Engine/EditorBlueprintResources/StandardMacros.IsValid` (`/Game/Component/Character/Stats/BPAC_StatsManager.ResourceStat` (`self.StatsManager`))
    (:`Is Valid`
      (switch `/Game/Enum/Support/E_Method_Action` Action
        (:`NewEnumerator1`
          (if (>= _returnvalue_2 (`self.MaxValue`))
            (set `self.Value` (`KismetMathLibrary.FMin` _returnvalue_2 (`self.MaxValue`)))
            (else
              (set `self.Value` _returnvalue_2)))
          (if (`self.IsEqualsValues?` (`self.MaxValue`) (`self.Value`))
            (`self.ValueIsMax`)))
        (:`NewEnumerator2`
          (if (<= _returnvalue (`self.MinValue`))
            (set `self.Value` (`KismetMathLibrary.FMax` _returnvalue (`self.MinValue`)))
            (else
              (set `self.Value` _returnvalue)))
          (if (`self.IsEqualsValues?` (`self.MinValue`) (`self.Value`))
            (`self.ValueIsMin`)))
        (:`NewEnumerator3`
          (if (<= Value (`self.MinValue`))
            (set `self.Value` (`self.MinValue`))
            (`self.ValueIsMin`)
            (elif (>= Value (`self.MaxValue`))
              (set `self.Value` (`self.MaxValue`))
              (`self.ValueIsMax`)
              (else
                (set `self.Value` Value)))))))))

(fn `IsEqualsValues?`
  (params (FirstValue :type "Float (double-precision)") (SecondValue :type "Float (double-precision)"))
  (returns (`IsEqual?` :type Boolean))
  (if (== FirstValue SecondValue)
    (return true)
    (else
      (return false))))

(fn `RegenerationResource`)

(fn `UserConstructionScript`)