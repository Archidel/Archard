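; Character health stat that tracks a clamped value, an injured state and health regeneration.
; ChangeValue adds, reduces or sets health, fires max and min events that only print debug text, then refreshes Injured against a threshold.
; When enabled, Tick regenerates health by delta time through ChangeValue, but only while health is above a stop-regen threshold and not yet at max.
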(event EventChangeValue
  (params (Value :type Float%20%28single-precision%29) (Action :type E_Method_Action%20Enum :default "NewEnumerator0"))
  (switch Utilities|FlowControl|Switch|SwitchonE_Method_Action Action
    (:NewEnumerator0
      _)
    (:NewEnumerator1
      (if (>= (+ (Variables|Health|GetValue) Value) (Variables|Health|GetMaxValue))
        (Variables|Health|SetValue (Math|Float|Min(Float) (+ (Variables|Health|GetValue) Value) (Variables|Health|GetMaxValue)))
        (else
          (Variables|Health|SetValue (+ (Variables|Health|GetValue) Value))))
      (if (Support|IsEqualsValues? (Variables|Health|GetMaxValue) (Variables|Health|GetValue))
        (CallFunction|ValueIsMax)))
    (:NewEnumerator2
      (if (<= (- (Variables|Health|GetValue) Value) (Variables|Health|GetMinValue))
        (Variables|Health|SetValue (Math|Float|Max(Float) (- (Variables|Health|GetValue) Value) (Variables|Health|GetMinValue)))
        (else
          (Variables|Health|SetValue (- (Variables|Health|GetValue) Value))))
      (if (Support|IsEqualsValues? (Variables|Health|GetMinValue) (Variables|Health|GetValue))
        (CallFunction|ValueIsMin)))
    (:NewEnumerator3
      (if (<= Value (Variables|Health|GetMinValue))
        (Variables|Health|SetValue (Variables|Health|GetMinValue))
        (CallFunction|ValueIsMin)
        (elif (>= Value (Variables|Health|GetMaxValue))
          (Variables|Health|SetValue (Variables|Health|GetMaxValue))
          (CallFunction|ValueIsMax)
          (else
            (Variables|Health|SetValue Value))))))
  (Injury|IsInjured?))

(event EventValueIsMax
  (Development|PrintString "Max"))

(event EventValueIsMin
  (Development|PrintString "Character is dead"))

(event EventTick
  (params (DeltaSeconds :type Float%20%28single-precision%29))
  (if (Variables|Regeneration|GetCanHealthRegen?)
    (CallFunction|RegenerationHealth)))

(fn ConstructionScript)

(fn IsEqualsValues?
  (params (FirstValue :type Float%20%28single-precision%29) (SecondValue :type Float%20%28single-precision%29))
  (if (== FirstValue SecondValue)
    (return true)
    (else
      (return false))))

(fn IsInjured?
  (if (<= (Variables|Health|GetValue) (|(({13F80A8A-4D09-00AC-5202-D4B41749FC68}*{33A852B8-4610-9385-5D4A-6BA56C794D1F})/100)))
    (Variables|Injury|SetInjured? true)
    (return true)
    (else
      (Variables|Injury|SetInjured? false)
      (return false))))

(fn RegenerationHealth
  (if (< (|(({EFECC46F-4888-FA34-81E5-1B8FE0539574}*{33A852B8-4610-9385-5D4A-6BA56C794D1F})/100)) (Variables|Health|GetValue))
    (if (not (Support|IsEqualsValues? (Variables|Health|GetValue) (Variables|Health|GetMaxValue)))
      (CallFunction|ChangeValue (* (Utilities|Time|GetWorldDeltaSeconds) (Variables|Regeneration|GetSpeedRegenHealth)) "NewEnumerator1"))))