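; Weight stat in the advanced character stat set, holding a value bounded between zero and MaxValue.
; ChangeVal applies Add or Reduce only when the result stays in range, rejecting out-of-range changes with an error message instead of clamping.
; CanChangeValue runs the same bounds checks without modifying the value.
; In both functions, the None and Change actions report an error and return false, as Change is not implemented.
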(fn `CanChangeValue?`
  (params (ActionType :type "/Game/Enum/Support/E_Method_Action Enum" :default "NewEnumerator0") (Value :type "Float (double-precision)"))
  (returns (`CanChange?` :type Boolean))
  (locals (L_Value :type "Float (double-precision)"))
  (set `local.L_Value` Value)
  (switch `/Game/Enum/Support/E_Method_Action` ActionType
    (:`NewEnumerator0`
      _)
    (:`NewEnumerator1`
      ;[1 1 1] Add
      (if (> (+ (`self.Value`) (`local.L_Value`)) (`self.MaxValue`))
        (return false)
        (else
          (return true))))
    (:`NewEnumerator2`
      ;[1 1 1] Reduce
      (if (< (- (`self.Value`) (`local.L_Value`)) 0.0)
        (return false)
        (else
          (return true))))
    (:`NewEnumerator3`
      _))
  (`/Game/Blueprint/Library/BML_ErrorMessanger.ErrorMessage` self "can change value aStats weight" "functionality is not implemented"
    (:`out`
      (return false))))

(fn `ChangeVal`
  (params (ActionType :type "/Game/Enum/Support/E_Method_Action Enum" :default "NewEnumerator0") (Value :type "Float (double-precision)"))
  (returns (`Success?` :type Boolean))
  (locals (L_Value :type "Float (double-precision)" :default 0.0))
  (bind _returnvalue (- (`self.Value`) (`local.L_Value`)))
  (bind _returnvalue_2 (+ (`self.Value`) (`local.L_Value`)))
  (set `local.L_Value` Value)
  (switch `/Game/Enum/Support/E_Method_Action` ActionType
    (:`NewEnumerator0`
      ;[1 1 1] None
      (`/Game/Blueprint/Library/BML_ErrorMessanger.ErrorMessage` self "change value astats weight" "None action method tye"
        (:`out`
          (return false))))
    (:`NewEnumerator1`
      ;[1 1 1] Add
      (if (> _returnvalue_2 (`self.MaxValue`))
        (`/Game/Blueprint/Library/BML_ErrorMessanger.ErrorMessage` self "Change value aStats weight" "In sum more then mxa value"
          (:`out`
            (return false)))
        (else
          (set `self.Value` _returnvalue_2)
          (return true))))
    (:`NewEnumerator2`
      ;[1 1 1] Reduce
      (if (< _returnvalue 0.0)
        (`/Game/Blueprint/Library/BML_ErrorMessanger.ErrorMessage` self "Change value aStats weight" "In sum less then 0"
          (:`out`
            (return false)))
        (else
          (set `self.Value` _returnvalue)
          (return true))))
    (:`NewEnumerator3`
      ;[1 1 1] None
      (`/Game/Blueprint/Library/BML_ErrorMessanger.ErrorMessage` self "change value astats weight" "Change functionality is not implemented"
        (:`out`
          (return false))))))

(fn `UserConstructionScript`
  (`parent.UserConstructionScript`))