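; Mana resource stat for the character stats system, which regenerates mana over time.
; Each tick, when regeneration is allowed and the value differs from its maximum, it calls RegenerationResource.
; That event passes the regen speed scaled by frame delta time to ChangeValue, keeping the rate frame-rate independent.
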(event `self.ReceiveTick`
  (params (DeltaSeconds :type "Float (single-precision)"))
  (if (`self.CanResourceRegen?`)
    (if (not (`self.IsEqualsValues?` (`self.Value`) (`self.MaxValue`)))
      (`self.RegenerationResource`))))

(event `self.RegenerationResource`
  (`self.ChangeValue` (* (`GameplayStatics.GetWorldDeltaSeconds`) (`self.SpeedRegenResource`)) "NewEnumerator1"))

(fn `UserConstructionScript`
  (`parent.UserConstructionScript`))