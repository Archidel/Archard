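; BP_StaminaStat holds a character stamina value kept between MinValue and MaxValue, with optional regeneration over time.
; Each Tick calls RegenerationStamina, which adds delta-time-scaled SpeedRegenStamina through ChangeValue when regeneration is allowed and stamina is below max.
; ChangeValue switches on an action to add, reduce or set the value, clamps it and fires ValueIsMax or ValueIsMin at the limits.
; Both limit events only print debug strings.
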(event `self.ReceiveTick`
  (params (DeltaSeconds :type "Float (single-precision)"))
  (`self.RegenerationStamina`))

(event `self.ValueIsMax`
  (`KismetSystemLibrary.PrintString` "Max"))

(event `self.ValueIsMin`
  (`KismetSystemLibrary.PrintString` "Min"))

(event `self.ChangeValue`
  (params (Value :type "Float (single-precision)") (Action :type "/Game/Enum/Support/E_Method_Action Enum" :default "NewEnumerator0"))
  (bind _returnvalue (- (`self.Value`) Value))
  (bind _returnvalue_2 (+ (`self.Value`) Value))
  (switch `/Game/Enum/Support/E_Method_Action` Action
    (:`NewEnumerator1`
      (if (>= _returnvalue_2 (`self.MaxValue`))
        (set `self.Value` (`KismetMathLibrary.FMin` _returnvalue_2 (`self.MaxValue`)))
        (else
          (set `self.Value` _returnvalue_2)))
      (if (`self.IsEqualsValues?` (`self.MaxValue`) (`self.Value`))
        (`self.ValueIsMax`)))
    (:`NewEnumerator2`
      (if (<= _returnvalue (`self.MinValue`))
        (set `self.Value` (`KismetMathLibrary.FMax` _returnvalue (`self.MinValue`)))
        (else
          (set `self.Value` _returnvalue)))
      (if (`self.IsEqualsValues?` (`self.MinValue`) (`self.Value`))
        (`self.ValueIsMin`)))
    (:`NewEnumerator3`
      (if (<= Value (`self.MinValue`))
        (set `self.Value` (`self.MinValue`))
        (`self.ValueIsMin`)
        (elif (>= Value (`self.MaxValue`))
          (set `self.Value` (`self.MaxValue`))
          (`self.ValueIsMax`)
          (else
            (set `self.Value` Value)))))))

(fn `IsEqualsValues?`
  (params (FirstValue :type "Float (double-precision)") (SecondValue :type "Float (double-precision)"))
  (returns (`IsEqual?` :type Boolean))
  (if (== FirstValue SecondValue)
    (return true)
    (else
      (return false))))

(fn `RegenerationStamina`
  (if (`self.CanRegenStamina`)
    (if (not (`self.IsEqualsValues?` (`self.Value`) (`self.MaxValue`)))
      (`self.ChangeValue` (* (`GameplayStatics.GetWorldDeltaSeconds`) (`self.SpeedRegenStamina`)) "NewEnumerator1"))))

(fn `UserConstructionScript`)