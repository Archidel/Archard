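; Athletics skill Blueprint that raises the Archard character's maximum stamina and walk speed.
; On Update, it casts the character to Archard and edits the stamina stat in BPACStatsManager and the CharacterMovement MaxWalkSpeed.
; Math expression nodes derive each bonus as a configurable percentage of the current value.
; Bonuses are added directly onto current values, so repeated updates compound.
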(event EventUpdate
  (bind (_success_ _character) (CallFunction|CastCharactertoArchard))
  (bind _bpac_statsmanager (Variables|/Game/Blueprint/Character/BPC_Character_Archard.BPC_Character_Archard_C|GetBPAC_StatsManager _character))
  (bind _charactermovement (Variables|/Script/Engine.Character|GetCharacterMovement _character))
  (bind _staminastat (Variables|/Game/Component/Character/Stats/BPAC_StatsManager.BPAC_StatsManager_C|GetStaminaStat _bpac_statsmanager))
  (if _success_
    (Variables|/Game/Blueprint/Character/Stats/BP_StaminaStat.BP_StaminaStat_C|SetMaxValue _staminastat (+ (|((MaxStamina*{18C71D20-4C2F-DDE2-763C-84BAEF031FCD})/100) (Variables|/Game/Blueprint/Character/Stats/BP_StaminaStat.BP_StaminaStat_C|GetMaxValue _staminastat)) (Variables|/Game/Blueprint/Character/Stats/BP_StaminaStat.BP_StaminaStat_C|GetMaxValue _staminastat)))
    (Variables|/Script/Engine.CharacterMovementComponent|SetMaxWalkSpeed _charactermovement (+ (|((Speed*{8E2D775C-4498-EE4F-47D8-F7ACEF42F1E2})/100) (Variables|/Script/Engine.CharacterMovementComponent|GetMaxWalkSpeed _charactermovement)) (Variables|/Script/Engine.CharacterMovementComponent|GetMaxWalkSpeed _charactermovement)))))

(fn ConstructionScript
  (|CallParentFunction))