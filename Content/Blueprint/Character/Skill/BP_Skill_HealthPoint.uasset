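; Health point skill that raises the Archard character's maximum health when its Update event runs.
; It casts the owning character to Archard, then feeds the stats manager's HealthStat max value through a percentage math expression and adds the result back.
; Each update therefore compounds on the already increased maximum, and only MaxValue is written.
; A failed cast reports through ErrorMessage.
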(event EventUpdate
  (bind (_success_ _character) (CallFunction|CastCharactertoArchard))
  (bind _bpac_statsmanager (Variables|/Game/Blueprint/Character/BPC_Character_Archard.BPC_Character_Archard_C|GetBPAC_StatsManager _character))
  (bind _healthstat (Variables|/Game/Component/Character/Stats/BPAC_StatsManager.BPAC_StatsManager_C|GetHealthStat _bpac_statsmanager))
  (if _success_
    (Variables|/Game/Blueprint/Character/Stats/BP_HealthStat.BP_HealthStat_C|SetMaxValue _healthstat (+ (|((CurrentHealth*{D2216E97-4EDB-915D-47D3-20815A2520ED})/100) (Variables|/Game/Blueprint/Character/Stats/BP_HealthStat.BP_HealthStat_C|GetMaxValue _healthstat)) (Variables|/Game/Blueprint/Character/Stats/BP_HealthStat.BP_HealthStat_C|GetMaxValue _healthstat)))
    (else
      (Utilities|ErrorMessage self "Event update" "Character cast failed to character archard"))))

(fn ConstructionScript
  (|CallParentFunction))