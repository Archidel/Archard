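; BP_Action is a character action Blueprint that runs through an action executor.
; OnTryExecuteAction stores the calling action component, asks BPACActionExecutor whether it can execute, and if so calls InitialExecuteAction to start it executing.
; OnCompiltedExecutingAction flags the executor as on cooldown and prints a debug message; this graph never clears that flag.
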(event `OnTryExecuteAction`
  (params (ActionComponent :type "/Game/Component/Character/Action/BPAC_ActionManager Object Reference"))
  (set `self.BPAC_ActionComponent` ActionComponent)
  (if (`/Game/Component/Character/Action/BPAC_ActionExecutor.CanExecuteAction?` (`self.BPAC_ActionExecutor`))
    (`self.InitialExecuteAction`)))

(event `InitialExecuteAction`
  (`/Game/Component/Character/Action/BPAC_ActionExecutor.Executing` (`self.BPAC_ActionExecutor`)))

(event `OnCompiltedExecutingAction`
  (set `/Game/Component/Character/Action/BPAC_ActionExecutor.OnCooldown` true (`self.BPAC_ActionExecutor`))
  (`KismetSystemLibrary.PrintString` "Executed"))

(fn `UserConstructionScript`)