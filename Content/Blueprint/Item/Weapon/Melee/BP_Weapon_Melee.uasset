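; Melee weapon item Blueprint that damages an AI character in front of whoever uses it.
; On use, it sphere-traces forward from the user's location on the Camera channel, ignoring the user, with reach scaled from the weapon's Length.
; If the hit actor is an AICharacter, it subtracts Damage directly from that character's Health.
; The trace's debug drawing is switched on, and construction only calls the parent.
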(event `/Game/Blueprint/Item/BP_Item.OnUsed`
  (params (Character :type "/Game/Blueprint/Character/BPC_Character_Archard Object Reference"))
  (bind _returnvalue (`self.K2_GetActorLocation` Character))
  (bind (_outhit _returnvalue_2) (`KismetSystemLibrary.SphereTraceSingle` _returnvalue (+ _returnvalue (* (`self.GetActorForwardVector` Character) (* (`KismetMathLibrary.Conv_IntToDouble` (`self.Length`)) 1.5))) 30.0 "TraceTypeQuery2" false (`|MakeArray` Character :!type "Actor Object Reference") "ForDuration"))
  (if _returnvalue_2
    (bind _asaicharacter (cast `/Game/AI/AICharacter` (`.HitActor` (`GameplayStatics.BreakHitResult` _outhit))))
    (set `/Game/AI/AICharacter.Health` (- (`/Game/AI/AICharacter.Health` _asaicharacter) (`self.Damage`)) _asaicharacter)))

(fn `UserConstructionScript`
  (`parent.UserConstructionScript`))