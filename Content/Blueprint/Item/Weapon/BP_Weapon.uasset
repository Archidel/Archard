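; BP_Weapon is a weapon item that a character picks up into its inventory by interacting with it.
; On Interact, if CanAddToInventory is set, it passes its own class, not the instance, to the character's BPACInventoryManager and destroys itself on success.
; A blocked or failed add reports through ErrorMessage and leaves the actor in place.
; The construction script only calls the parent's.
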(event `/Game/Interface/Character/Interact/BPI_Interact.Interact`
  (params (Character :type "/Game/Blueprint/Character/BPC_Character_Archard Object Reference"))
  (if (`self.CanAddToInventory`)
    (bind _success_ (`/Game/Component/Character/Inventory/BPAC_InventoryManager.AddItemToInventory` (`/Game/Blueprint/Character/BPC_Character_Archard.BPAC_InventoryManager` Character) (`GameplayStatics.GetObjectClass` self)))
    (if _success_
      (`self.K2_DestroyActor` self)
      (else
        (`/Game/Blueprint/Library/BML_ErrorMessanger.ErrorMessage` self "event graph" "error of adding to inventory")))
    (else
      (`/Game/Blueprint/Library/BML_ErrorMessanger.ErrorMessage` self "event graph" "we cant add to inventory"))))

(fn `UserConstructionScript`
  (`parent.UserConstructionScript`))