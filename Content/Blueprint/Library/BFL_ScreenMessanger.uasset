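; Blueprint function library that shows an animated message in the center of the screen.
; CenterScreenMessage switches on a status to pick the caller's color or a preset error, warning or success color.
; Each branch creates a new WB_ScreenMessanger_Center widget with the message and color, adds it to the viewport and plays its message animation.
; Unwired nodes for removing widgets when the animation finishes never run.
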(fn `CenterScreenMessage`
  (params (Status :type "/Game/Enum/Character/ScreenMessenger/E_MessageStatus Enum" :default "NewEnumerator0") (Message :type Text) (Color :type "LinearColor Structure" :default (struct :`R` 1.0 :`G` 1.0 :`B` 1.0 :`A` 1.0)))
  (locals (SuccessColor :type "LinearColor Structure" :default (struct :`R` 0.081043 :`G` 1.0 :`A` 1.0)) (WarningColor :type "LinearColor Structure" :default (struct :`R` 0.953125 :`G` 0.72833 :`B` 0.243245 :`A` 1.0)) (ErrorColor :type "LinearColor Structure" :default (struct :`R` 1.0 :`A` 1.0)))
  (switch `/Game/Enum/Character/ScreenMessenger/E_MessageStatus` Status
    (:`NewEnumerator0`
      (bind _returnvalue (`|CreateWidget` "/Game/Widget/Character/ScreenMessenger/WB_ScreenMessanger_Center.WB_ScreenMessanger_Center_C" null Color Message))
      (`UserWidget.AddToViewport` _returnvalue 0)
      (`UserWidget.PlayAnimation` _returnvalue (`/Game/Widget/Character/ScreenMessenger/WB_ScreenMessanger_Center.MessageAnimation` _returnvalue) 0.0 1 "Forward" 1.0))
    (:`NewEnumerator1`
      (bind _returnvalue_2 (`|CreateWidget` "/Game/Widget/Character/ScreenMessenger/WB_ScreenMessanger_Center.WB_ScreenMessanger_Center_C" null (`local.ErrorColor`) Message))
      (`UserWidget.AddToViewport` _returnvalue_2 0)
      (`UserWidget.PlayAnimation` _returnvalue_2 (`/Game/Widget/Character/ScreenMessenger/WB_ScreenMessanger_Center.MessageAnimation` _returnvalue_2) 0.0 1 "Forward" 1.0))
    (:`NewEnumerator2`
      (bind _returnvalue_3 (`|CreateWidget` "/Game/Widget/Character/ScreenMessenger/WB_ScreenMessanger_Center.WB_ScreenMessanger_Center_C" null (`local.WarningColor`) Message))
      (`UserWidget.AddToViewport` _returnvalue_3 0)
      (`UserWidget.PlayAnimation` _returnvalue_3 (`/Game/Widget/Character/ScreenMessenger/WB_ScreenMessanger_Center.MessageAnimation` _returnvalue_3) 0.0 1 "Forward" 1.0))
    (:`NewEnumerator3`
      (bind _returnvalue_4 (`|CreateWidget` "/Game/Widget/Character/ScreenMessenger/WB_ScreenMessanger_Center.WB_ScreenMessanger_Center_C" null (`local.SuccessColor`) Message))
      (`UserWidget.AddToViewport` _returnvalue_4 0)
      (`UserWidget.PlayAnimation` _returnvalue_4 (`/Game/Widget/Character/ScreenMessenger/WB_ScreenMessanger_Center.MessageAnimation` _returnvalue_4) 0.0 1 "Forward" 1.0))))